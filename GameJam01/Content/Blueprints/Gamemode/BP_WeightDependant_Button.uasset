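; BP_WeightDependant_Button is a pressure button that triggers when enough possessable-pawn weight rests on it.
; Its WeightDetector overlap events keep a list of BP_Master_Possessable_pawn actors and re-sum their Weight on every change.
; Reaching WeightNeeded fires Execute through a DoOnce, which resets only when a weight check falls below the threshold.
; Execute currently just prints a debug message.
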(event OnComponentBeginOverlap(WeightDetector)
  (params (OverlappedComponent :type Primitive%20Component%20Object%20Reference) (OtherActor :type Actor%20Object%20Reference) (OtherComp :type Primitive%20Component%20Object%20Reference) (OtherBodyIndex :type Integer) (bFromSweep :type Boolean) (SweepResult :type Hit%20Result%20Structure%20%28by%20ref%29))
  (bind _collectedpawns (Variables|Default|GetCollectedPawns))
  (bind _asbp_master_possessable_pawn (Utilities|Casting|CastToBP_Master_Possessable_pawn OtherActor))
  (if (not (Utilities|Array|ContainsItem _collectedpawns _asbp_master_possessable_pawn))
    (Utilities|Array|AddUnique _collectedpawns _asbp_master_possessable_pawn)
    (CallFunction|CheckWeight)))

(event OnComponentEndOverlap(WeightDetector)
  (params (OverlappedComponent :type Primitive%20Component%20Object%20Reference) (OtherActor :type Actor%20Object%20Reference) (OtherComp :type Primitive%20Component%20Object%20Reference) (OtherBodyIndex :type Integer))
  (bind _asbp_master_possessable_pawn (Utilities|Casting|CastToBP_Master_Possessable_pawn OtherActor))
  (Utilities|Array|RemoveItem (Variables|Default|GetCollectedPawns) _asbp_master_possessable_pawn)
  (CallFunction|CheckWeight))

(event Custom|CheckWeight
  (Variables|Default|SetCurrentWeight 0.0)
  (for _array_element (Variables|Default|GetCollectedPawns)
    (bind _output_get (Variables|Default|SetCurrentWeight (+ (Variables|Default|GetCurrentWeight) (Variables|/Game/Blueprints/Possessable_pawns/BP_Master_Possessable_pawn.BP_Master_Possessable_pawn_C|GetWeight _array_element))))
    (Development|PrintString (Utilities|String|ToString(Float) _output_get)))
  (if (>= (Variables|Default|GetCurrentWeight) (Variables|Default|GetWeightNeeded))
    (Utilities|FlowControl|DoOnce false :!label _label
      (:Completed
        (CallFunction|Execute)))
    (else
      (goto _label Reset))))

(event Custom|Execute
  (Development|PrintString "ButtonHasBeenPushed!" true true "(R=0.000000,G=0.660000,B=1.000000,A=1.000000)" 5.0))

(event EventBeginPlay)

(event Collision|EventActorBeginOverlap
  (params (OtherActor :type Actor%20Object%20Reference)))

(event EventTick
  (params (DeltaSeconds :type Float%20%28single-precision%29)))

(fn ConstructionScript)